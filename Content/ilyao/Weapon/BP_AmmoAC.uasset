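; BP_AmmoAC is an ammo component that tracks the current ammunition count for a weapon.
; CurrentAmmo fills to MaxAmmo on BeginPlay.
; SubstrutAmmo deducts a given amount and clamps the result between zero and MaxAmmo, while ChekAmmo reports whether enough ammo remains for a requested amount.
; It contains no reload logic, and subtraction does not itself call the check.
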(event `self.ReceiveBeginPlay`
  (set `self.CurrentAmmo` (`self.MaxAmmo`)))

(fn `Chek Ammo`
  (params (Value :type Integer :default 1))
  (returns (ReturnValue :type Boolean))
  (return (>= (`self.CurrentAmmo`) Value)))

(fn `SubstrutAmmo`
  (params (Value :type Integer :default 1))
  (set `self.CurrentAmmo` (`KismetMathLibrary.Clamp` (- (`self.CurrentAmmo`) Value) 0 (`self.MaxAmmo`))))