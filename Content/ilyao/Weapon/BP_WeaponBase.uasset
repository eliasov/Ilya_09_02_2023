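; Base weapon actor that fires automatically every two seconds from BeginPlay, looping through a Replay event back into the delay.
; Each shot checks and deducts one round in the BPAmmoAC component, then spawns a BP_AmmoBase projectile at the Arrow's transform.
; Without enough ammo it plays a sound at the actor's location instead.
; Every firing attempt refreshes a TextRender showing current and maximum ammo.
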(event `self.ReceiveBeginPlay`
  (`KismetSystemLibrary.Delay` 2.0 :!label _label)
  (`self.Fire`)
  (`self.Replay`))

(event `Replay`
  (goto _label))

(event `Fire`
  (bind _bp_ammoac (`self.BP_AmmoAC`))
  ;[1 1 1] Спавн снарядов
  (`|ExecutionSequence`
    (:`then_0`
      (if (`/Game/ilyao/Weapon/BP_AmmoAC.Chek Ammo` _bp_ammoac 1)
        (`/Game/ilyao/Weapon/BP_AmmoAC.SubstrutAmmo` _bp_ammoac 1)
        (`|SpawnActorFromClass` "/Game/ilyao/Weapon/BP_AmmoBase.BP_AmmoBase_C" (`SceneComponent.K2_GetComponentToWorld` (`self.Arrow`)) "AlwaysSpawn" "OverrideRootScale" null null)
        (else
          (`GameplayStatics.SpawnSoundAtLocation` "/Game/Download/StarterContent/Audio/Light01.Light01" (`self.K2_GetActorLocation`) (struct) 1.0 1.0 0.0 null null))))
    (:`then_1`
      (`TextRenderComponent.K2_SetText` (`self.TextRender`) (`|FormatText` "{Current}/{Max}" (`/Game/ilyao/Weapon/BP_AmmoAC.CurrentAmmo` (`self.BP_AmmoAC`)) (`/Game/ilyao/Weapon/BP_AmmoAC.MaxAmmo` (`self.BP_AmmoAC`)))))))

(fn `UserConstructionScript`)